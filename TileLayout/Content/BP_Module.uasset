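; BP_Module is a grid tile actor that picks its texture at construction from the tiles allowed at its location.
; The construction script looks up its exact XY position in SlotLayout's SlotIndex map and collects the indices flagged in AvailableTiles.
; A seeded stream chooses one index into TextureArray, which feeds the Tile parameter of a dynamic M_Tile material on the Plane.
; It prints the candidate indices, or a message when off-grid or without a layout.
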(event EventBeginPlay)

(event Collision|EventActorBeginOverlap
  (params (OtherActor :type Actor%20Object%20Reference)))

(event EventTick
  (params (DeltaSeconds :type Float%20%28single-precision%29)))

(fn ConstructionScript
  (bind _returnvalue (Transformation|GetActorLocation))
  (bind _slotlayout (Variables|Default|GetSlotLayout))
  (bind _options (Variables|Default|GetOptions))
  (bind _slotindex (Variables|/Game/BP_SlotLayout.BP_SlotLayout_C|GetSlotIndex _slotlayout))
  (bind (_value _returnvalue_2) (Utilities|Map|Find _slotindex (Math|Vector2D|MakeVector2D (.x _returnvalue) (.y _returnvalue))))
  (bind _returnvalue_3 (Rendering|Material|CreateDynamicMaterialInstance "/Game/M_Tile.M_Tile" "TileMat" :!class /Script/Engine.KismetMaterialLibrary))
  (Variables|Default|SetTileMat _returnvalue_3)
  (Rendering|Material|SetMaterial (Variables|Default|GetPlane) 0 _returnvalue_3)
  (Utilities|IsValid (Variables|Default|GetSlotLayout)
    (:Is%20Valid
      (if _returnvalue_2
        (for (_array_element _array_index) (Variables|/Game/BP_Slot.BP_Slot_C|GetAvailableTiles _value)
          (if _array_element
            (Utilities|Array|Add (Variables|Default|GetOptions) _array_index)))
        (for _array_element_2 _options
          (Development|PrintString (Utilities|String|ToString(Integer) _array_element_2)))
        (Rendering|Material|SetTextureParameterValue (Variables|Default|GetTileMat) "Tile" (Utilities|Array|Get(acopy) (Variables|Default|GetTextureArray) (Utilities|Array|Get(acopy) _options (Math|Random|RandomIntegerinRangefromStream 0 (- (Utilities|Array|Length _options) 1) (Variables|Default|GetSeed)))))
        (else
          (Development|PrintString "OffGrid"))))
    (:Is%20Not%20Valid
      (Development|PrintString "SlotLayout Not designated"))))